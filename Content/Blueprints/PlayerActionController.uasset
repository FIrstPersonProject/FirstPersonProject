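; Player action actor that lets the first-person character spawn and temporarily possess a mouse or flying character.
; Keys 1 and 2 spawn and possess one of each, passing its reference to the original character.
; R or a Tick-driven timer returns control to that character, telling the flyer to land.
; E destroys a spawned creature when the unpossessed player overlaps it, allowing a respawn.
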(event EventBeginPlay
  ;[1 1 1] Store player's original character so we can jump back to it
  (Variables|Default|SetPlayerOrigChar (Game|GetPlayerCharacter 0))
  (Input|EnableInput (Game|GetPlayerController 0)))

(event EventActorBeginOverlap
  (params (OtherActor :type Actor%20Object%20Reference)))

(event EventTick
  (params (DeltaSeconds :type Float%20%28single-precision%29))
  ;[1 1 1] Timed Possession
  (bind _output_get (Variables|HelperBot|SetPossessionTimer (+ DeltaSeconds (Variables|HelperBot|GetPossessionTimer))))
  (if (and (>= _output_get (Variables|HelperBot|GetMaxPossessionTime)) (Variables|HelperBot|GetMouseSpawned))
    ;[1 1 1] Unpossessing MouseChar Automatically
    (if (Variables|HelperBot|GetPossessEnabled)
      (Variables|HelperBot|SetPossessEnabled false)
      (Pawn|Possess (Game|GetPlayerController 0) (Variables|Default|GetPlayerOrigChar)))
    (elif (and (Variables|HelperBot|GetFlyerSpawned) (>= _output_get (Variables|HelperBot|GetMaxPossessionTime)))
      ;[1 1 1] Unpossessing FlyingChar Automatically
      (if (Variables|HelperBot|GetPossessEnabled)
        (Variables|HelperBot|SetPossessEnabled false)
        (Pawn|Possess (Game|GetPlayerController 0) (Variables|Default|GetPlayerOrigChar))
        (bind _asflying_char (Utilities|Casting|CastToFlyingChar (Variables|HelperBot|GetSpawnedFlyer)))
        (Variables|/Game/FirstPersonBP/Blueprints/FlyingChar.FlyingChar_C|SetLand _asflying_char true)))))

(event Input|KeyboardEvents|R
  ;[1 1 1] Unpossessing FlyingChar
  (:Released
    (if (Variables|HelperBot|GetPossessEnabled)
      (if (Variables|HelperBot|GetFlyerSpawned)
        (Variables|HelperBot|SetPossessEnabled false)
        (Pawn|Possess (Game|GetPlayerController 0) (Variables|Default|GetPlayerOrigChar))
        (bind _asflying_char (Utilities|Casting|CastToFlyingChar (Variables|HelperBot|GetSpawnedFlyer)))
        (Variables|/Game/FirstPersonBP/Blueprints/FlyingChar.FlyingChar_C|SetLand _asflying_char true)))))

(event Input|KeyboardEvents|R
  ;[1 1 1] Unpossessing MouseChar
  (:Released
    (if (Variables|HelperBot|GetPossessEnabled)
      (if (Variables|HelperBot|GetMouseSpawned)
        (Variables|HelperBot|SetPossessEnabled false)
        (Pawn|Possess (Game|GetPlayerController 0) (Variables|Default|GetPlayerOrigChar))))))

(event Input|KeyboardEvents|2
  (bind _returnvalue (Game|GetPlayerCharacter 0))
  ;[1 1 1] Spawning FlyingChar
  (:Released
    (if (not (Variables|HelperBot|GetPossessEnabled))
      (if (not (Variables|HelperBot|GetFlyerSpawned))
        (bind _returnvalue_2 (Game|SpawnActorfromClass "/Game/FirstPersonBP/Blueprints/FlyingChar.FlyingChar_C" (Math|Transform|ComposeTransforms (Math|Conversions|ToTransform(Vector) (+ (Transformation|GetActorForwardVector _returnvalue) "100.000000, 0, 0")) (Transformation|GetActorTransform _returnvalue)) false false 0))
        (Variables|HelperBot|SetSpawnedFlyer _returnvalue_2)
        (Variables|HelperBot|SetFlyerSpawned true)
        (bind _asfirst_person_character (Utilities|Casting|CastToFirstPersonCharacter (Variables|Default|GetPlayerOrigChar)))
        (Variables|/Game/FirstPersonBP/Blueprints/FirstPersonCharacter.FirstPersonCharacter_C|SetFlyingCharRef _asfirst_person_character (Variables|HelperBot|GetSpawnedFlyer))
        ;[1 1 1] Posessing flying pawn
        (if (Variables|HelperBot|GetFlyerSpawned)
          (Variables|HelperBot|SetPossessEnabled true)
          (Pawn|Possess (Game|GetPlayerController 0) (Variables|HelperBot|GetSpawnedFlyer))
          (Variables|HelperBot|SetPossessionTimer 0.0))))))

(event Input|KeyboardEvents|1
  (bind _returnvalue (Game|GetPlayerCharacter 0))
  ;[1 1 1] Spawning MouseChar
  (:Released
    (if (not (Variables|HelperBot|GetPossessEnabled))
      (if (not (Variables|HelperBot|GetMouseSpawned))
        (bind _returnvalue_2 (Game|SpawnActorfromClass "/Game/FirstPersonBP/Blueprints/MouseChar.MouseChar_C" (Math|Transform|ComposeTransforms (Math|Conversions|ToTransform(Vector) (+ (Transformation|GetActorForwardVector _returnvalue) "100.000000,0.000000,0.000000")) (Transformation|GetActorTransform _returnvalue)) false 0))
        (Variables|HelperBot|SetSpawnedMouse _returnvalue_2)
        (Variables|HelperBot|SetMouseSpawned true)
        (bind _asfirst_person_character (Utilities|Casting|CastToFirstPersonCharacter (Variables|Default|GetPlayerOrigChar)))
        (Variables|/Game/FirstPersonBP/Blueprints/FirstPersonCharacter.FirstPersonCharacter_C|SetMouseCharRef _asfirst_person_character (Variables|HelperBot|GetSpawnedMouse))
        ;[1 1 1] Posessing mouse pawn
        (if (Variables|HelperBot|GetMouseSpawned)
          (Variables|HelperBot|SetPossessEnabled true)
          (Pawn|Possess (Game|GetPlayerController 0) (Variables|HelperBot|GetSpawnedMouse))
          (Variables|HelperBot|SetPossessionTimer 0.0))))))

(event Input|KeyboardEvents|E
  ;[1 1 1] Destroying FlyingChar
  (:Released
    (if (not (Variables|HelperBot|GetPossessEnabled))
      (if (Variables|HelperBot|GetFlyerSpawned)
        (bind _asfirst_person_character (Utilities|Casting|CastToFirstPersonCharacter (Variables|Default|GetPlayerOrigChar)))
        (if (Variables|/Game/FirstPersonBP/Blueprints/FirstPersonCharacter.FirstPersonCharacter_C|GetPlayerOverlappingFlyer _asfirst_person_character)
          (Actor|DestroyActor (Variables|HelperBot|GetSpawnedFlyer))
          (Variables|HelperBot|SetFlyerSpawned false))))))

(event Input|KeyboardEvents|E
  ;[1 1 1] Destroying MouseChar
  (:Released
    (if (not (Variables|HelperBot|GetPossessEnabled))
      (if (Variables|HelperBot|GetMouseSpawned)
        (bind _asfirst_person_character (Utilities|Casting|CastToFirstPersonCharacter (Variables|Default|GetPlayerOrigChar)))
        (if (Variables|/Game/FirstPersonBP/Blueprints/FirstPersonCharacter.FirstPersonCharacter_C|GetPlayerOverlappingMouse _asfirst_person_character)
          (Actor|DestroyActor (Variables|HelperBot|GetSpawnedMouse))
          (Variables|HelperBot|SetMouseSpawned false))))))

(fn ConstructionScript)