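; ResetButton is an interactable button that switches off alarms on a configured set of Blueprints.
; It enables input from the first player controller on BeginPlay and listens for the E key release.
; If the player character overlaps ButtonCollision on release, it loops through BlueprintsToReset and calls SendAlarmMessage with false on each entry.
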(event EventBeginPlay
  ;[1 1 1] Enable input
  (Input|EnableInput (Game|GetPlayerController 0)))

(event EventTick
  (params (DeltaSeconds :type Float%20%28single-precision%29)))

(event Input|KeyboardEvents|E
  (bind _blueprintstoreset (Variables|Default|GetBlueprintsToReset))
  (:Released
    (if (Utilities|Array|ContainsItem (Collision|GetOverlappingActors (Variables|Default|GetButtonCollision) "/Script/Engine.Character" :!class /Script/Engine.PrimitiveComponent) (Game|GetPlayerCharacter 0))
      (for _index (range 0 (- (Utilities|Array|Length _blueprintstoreset) 1))
        (Class|AlarmInterface|SendAlarm(Message) (Utilities|Array|Get(acopy) _blueprintstoreset _index) false)))))

(fn ConstructionScript)