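; BP_SecurityDoor is a door that reacts to an alarm by moving its mesh vertically.
; BeginPlay caches the mesh's world location and rotation as the original transform.
; SendAlarm uses MoveComponentTo to lower the mesh 300 units over three seconds when alarmed, and returns it to the original transform otherwise.
; The cached world-space values serve as relative-space move targets.
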(event EventBeginPlay
  (bind _temp_door_staticmesh (Variables|Default|GetTemp_Door_StaticMesh))
  (Variables|Default|SetoriginalPosition (Transformation|GetWorldLocation _temp_door_staticmesh))
  (Variables|Default|SetoriginalRotation (Transformation|GetWorldRotation _temp_door_staticmesh)))

(event EventActorBeginOverlap
  (params (OtherActor :type Actor%20Object%20Reference)))

(event EventTick
  (params (DeltaSeconds :type Float%20%28single-precision%29)))

(event EventSendAlarm
  (params (Alarmed :type Boolean))
  (bind _originalposition (Variables|Default|GetoriginalPosition))
  (bind _temp_door_staticmesh (Variables|Default|GetTemp_Door_StaticMesh))
  (bind (_x _y _z) (Math|Vector|BreakVector _originalposition))
  (if Alarmed
    (Components|MoveComponentTo _temp_door_staticmesh (Math|Vector|MakeVector _x _y (- _z 3e+02)) (Variables|Default|GetoriginalRotation) false false 3.0)
    (else
      (Components|MoveComponentTo _temp_door_staticmesh (Variables|Default|GetoriginalPosition) (Variables|Default|GetoriginalRotation) false false 0.2))))

(fn ConstructionScript)