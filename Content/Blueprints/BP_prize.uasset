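; BP_prize is a pickup actor that records that the player has the item needed by the level-end script.
; Box overlap events toggle an IsOverlapping flag for any actor, and input from player controller 0 is enabled on BeginPlay.
; Pressing E while overlapping sets PlayerHasItem on the LevelEndScript reference and hides the prize in game without destroying it.
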(event OnComponentEndOverlap(Box)
  (params (OtherActor :type Actor%20Object%20Reference) (OtherComp :type Primitive%20Component%20Object%20Reference) (OtherBodyIndex :type Integer))
  (Variables|Default|SetisOverlapping false))

(event OnComponentBeginOverlap(Box)
  (params (OtherActor :type Actor%20Object%20Reference) (OtherComp :type Primitive%20Component%20Object%20Reference) (OtherBodyIndex :type Integer) (bFromSweep :type Boolean) (SweepResult :type Hit%20Result%20Structure%20%28by%20ref%29))
  (Variables|Default|SetisOverlapping true))

(event EventBeginPlay
  (Input|EnableInput (Game|GetPlayerController 0)))

(event EventTick
  (params (DeltaSeconds :type Float%20%28single-precision%29)))

(event Input|KeyboardEvents|E
  (:Pressed
    (if (Variables|Default|GetisOverlapping)
      (Variables|/Game/Blueprints/LevelEndCheck.LevelEndCheck_C|SetplayerHasItem (Variables|Default|GetLevel%20End%20Script) true)
      (Rendering|SetActorHiddenInGame true))))

(fn ConstructionScript)