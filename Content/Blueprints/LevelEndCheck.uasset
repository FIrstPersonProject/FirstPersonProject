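; Level exit actor that ends the level when the first-person character, with the PlayerHasItem flag set, stands in its LevelEndTrigger.
; Tick polls the trigger's overlaps, then sets LevelEnd, shows a HUD message and starts a short timer for ChangeLevel, which opens level1-1.
; The timer is set again every tick during overlap, so its countdown keeps restarting while the character remains inside.
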(event EventBeginPlay)

(event EventActorBeginOverlap
  (params (OtherActor :type Actor%20Object%20Reference)))

(event EventTick
  (params (DeltaSeconds :type Float%20%28single-precision%29))
  (if (Variables|Default|GetplayerHasItem)
    (bind _array_element (Utilities|Array|ForEachLoopwithBreak (Collision|GetOverlappingActors (Variables|Default|GetLevel%20End%20Trigger) "/Game/FirstPersonBP/Blueprints/FirstPersonCharacter.FirstPersonCharacter_C" :!class /Script/Engine.Actor))
      (:LoopBody
        (Utilities|Casting|CastToFirstPersonCharacter _array_element)
        (Utilities|Time|SetTimerbyFunctionName 0 "ChangeLevel" 2.0)
        (Variables|Default|SetLevelEnd true)
        (Class|LevelComplete|ShowText(Message) (HUD|GetHUD (Game|GetPlayerController 0)) true)))))

(fn ConstructionScript)

(fn ChangeLevel
  (Game|OpenLevel(byName) "level1-1"))