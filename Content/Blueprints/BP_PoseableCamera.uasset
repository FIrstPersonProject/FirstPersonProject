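; Security camera that sweeps a poseable mesh bone back and forth and alerts linked Blueprints when it spots the player.
; A timeline drives the bone's world yaw, with the spotlight and detection capsule attached and re-oriented on each update.
; Player overlap pauses the sweep; timeline updates also set the dynamic material's color blend and send alarm messages if active.
; Enable and disable events toggle detection and playback.
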(event EventBeginPlay
  (bind _poseablemesh (Variables|Default|GetPoseableMesh))
  (bind _poseablemesh_2 (Variables|Default|GetPoseableMesh))
  (bind _blueprintstoalert (Variables|Default|GetBlueprintsToAlert))
  (bind _returnvalue (Transformation|GetSocketRotation _poseablemesh_2 "Bone_002"))
  (bind (_pitch _yaw _roll) (Class|KismetMathLibrary|BreakRot _returnvalue))
  (Class|SceneComponent|Attachto (Variables|Default|GetSpotLight) _poseablemesh "Bone_002" "KeepWorldPosition" false)
  (Class|SceneComponent|Attachto (Variables|Default|GetOverlapCapsule) _poseablemesh "Bone_002" "KeepWorldPosition" false)
  (bind _angle_multiplier (Timeline|rotate%20camera PlayFromStart)
    (:Update
      (Variables|Default|SetCameraNewRotation (Class|KismetMathLibrary|MakeRot _pitch (+ (* _angle_multiplier (Variables|Default|Getcamera%20max%20angle)) (Variables|Default|GetCameraFacingDirection)) _roll))
      (Components|PoseableMesh|SetBoneRotationbyName "Bone_002" (Variables|Default|GetCameraNewRotation) "WorldSpace")
      (Transformation|SetWorldRotation (Variables|Default|GetOverlapCapsule) (Class|KismetMathLibrary|MakeRot (.Pitch (Class|KismetMathLibrary|BreakRot (Variables|Default|GetCameraNewRotation))) (.Yaw (Class|KismetMathLibrary|BreakRot (Variables|Default|GetCameraNewRotation))) (+ (.Roll (Class|KismetMathLibrary|BreakRot (Variables|Default|GetCameraNewRotation))) 2e+01)) false)
      (Transformation|SetWorldRotation (Variables|Default|GetSpotLight) (Class|KismetMathLibrary|MakeRot (- (.Pitch (Class|KismetMathLibrary|BreakRot (Variables|Default|GetCameraNewRotation))) 35.0) (+ (.Yaw (Class|KismetMathLibrary|BreakRot (Variables|Default|GetCameraNewRotation))) 85.0) (.Roll (Class|KismetMathLibrary|BreakRot (Variables|Default|GetCameraNewRotation)))) false)
      ;[1 1 1] Change dynamic material instance's color
      (Rendering|Material|SetScalarParameterValue (Variables|Default|GetDynMat) "Lerp Alpha" (Math|Float|SelectFloat 1.0 0.0 (and (Variables|Default|GetPlayerIsOverlapping) (Variables|Default|GetisActive))) :!class /Script/Engine.MaterialInstanceDynamic)
      (if (and (Variables|Default|GetPlayerIsOverlapping) (Variables|Default|GetisActive))
        (for _index (range 0 (- (Utilities|Array|Length _blueprintstoalert) 1))
          (Class|AlarmInterface|SendAlarm(Message) (Utilities|Array|Get(acopy) _blueprintstoalert _index) true))))))

(event EventActorBeginOverlap
  (params (OtherActor :type Actor%20Object%20Reference))
  (bind _poseablemesh (Variables|Default|GetPoseableMesh))
  (bind _blueprintstoalert (Variables|Default|GetBlueprintsToAlert))
  (bind _returnvalue (Transformation|GetSocketRotation _poseablemesh "Bone_002"))
  (bind (_pitch _yaw _roll) (Class|KismetMathLibrary|BreakRot _returnvalue))
  (if (== OtherActor (Game|GetPlayerCharacter 0))
    (Variables|Default|SetPlayerIsOverlapping true)
    (bind _angle_multiplier (Timeline|rotate%20camera Stop)
      (:Update
        (Variables|Default|SetCameraNewRotation (Class|KismetMathLibrary|MakeRot _pitch (+ (* _angle_multiplier (Variables|Default|Getcamera%20max%20angle)) (Variables|Default|GetCameraFacingDirection)) _roll))
        (Components|PoseableMesh|SetBoneRotationbyName "Bone_002" (Variables|Default|GetCameraNewRotation) "WorldSpace")
        (Transformation|SetWorldRotation (Variables|Default|GetOverlapCapsule) (Class|KismetMathLibrary|MakeRot (.Pitch (Class|KismetMathLibrary|BreakRot (Variables|Default|GetCameraNewRotation))) (.Yaw (Class|KismetMathLibrary|BreakRot (Variables|Default|GetCameraNewRotation))) (+ (.Roll (Class|KismetMathLibrary|BreakRot (Variables|Default|GetCameraNewRotation))) 2e+01)) false)
        (Transformation|SetWorldRotation (Variables|Default|GetSpotLight) (Class|KismetMathLibrary|MakeRot (- (.Pitch (Class|KismetMathLibrary|BreakRot (Variables|Default|GetCameraNewRotation))) 35.0) (+ (.Yaw (Class|KismetMathLibrary|BreakRot (Variables|Default|GetCameraNewRotation))) 85.0) (.Roll (Class|KismetMathLibrary|BreakRot (Variables|Default|GetCameraNewRotation)))) false)
        ;[1 1 1] Change dynamic material instance's color
        (Rendering|Material|SetScalarParameterValue (Variables|Default|GetDynMat) "Lerp Alpha" (Math|Float|SelectFloat 1.0 0.0 (and (Variables|Default|GetPlayerIsOverlapping) (Variables|Default|GetisActive))) :!class /Script/Engine.MaterialInstanceDynamic)
        (if (and (Variables|Default|GetPlayerIsOverlapping) (Variables|Default|GetisActive))
          (for _index (range 0 (- (Utilities|Array|Length _blueprintstoalert) 1))
            (Class|AlarmInterface|SendAlarm(Message) (Utilities|Array|Get(acopy) _blueprintstoalert _index) true)))))))

(event EventSetEnabled
  (Variables|Default|SetisActive true)
  (Audio|Components|Audio|Play))

(event EventSetDisabled
  (Variables|Default|SetisActive false)
  (Audio|Components|Audio|Stop))

(event EventActorEndOverlap
  (params (OtherActor :type Actor%20Object%20Reference))
  (bind _poseablemesh (Variables|Default|GetPoseableMesh))
  (bind _blueprintstoalert (Variables|Default|GetBlueprintsToAlert))
  (bind _returnvalue (Transformation|GetSocketRotation _poseablemesh "Bone_002"))
  (bind (_pitch _yaw _roll) (Class|KismetMathLibrary|BreakRot _returnvalue))
  (if (== OtherActor (Game|GetPlayerCharacter 0))
    (Variables|Default|SetPlayerIsOverlapping false)
    (bind _angle_multiplier (Timeline|rotate%20camera Play)
      (:Update
        (Variables|Default|SetCameraNewRotation (Class|KismetMathLibrary|MakeRot _pitch (+ (* _angle_multiplier (Variables|Default|Getcamera%20max%20angle)) (Variables|Default|GetCameraFacingDirection)) _roll))
        (Components|PoseableMesh|SetBoneRotationbyName "Bone_002" (Variables|Default|GetCameraNewRotation) "WorldSpace")
        (Transformation|SetWorldRotation (Variables|Default|GetOverlapCapsule) (Class|KismetMathLibrary|MakeRot (.Pitch (Class|KismetMathLibrary|BreakRot (Variables|Default|GetCameraNewRotation))) (.Yaw (Class|KismetMathLibrary|BreakRot (Variables|Default|GetCameraNewRotation))) (+ (.Roll (Class|KismetMathLibrary|BreakRot (Variables|Default|GetCameraNewRotation))) 2e+01)) false)
        (Transformation|SetWorldRotation (Variables|Default|GetSpotLight) (Class|KismetMathLibrary|MakeRot (- (.Pitch (Class|KismetMathLibrary|BreakRot (Variables|Default|GetCameraNewRotation))) 35.0) (+ (.Yaw (Class|KismetMathLibrary|BreakRot (Variables|Default|GetCameraNewRotation))) 85.0) (.Roll (Class|KismetMathLibrary|BreakRot (Variables|Default|GetCameraNewRotation)))) false)
        ;[1 1 1] Change dynamic material instance's color
        (Rendering|Material|SetScalarParameterValue (Variables|Default|GetDynMat) "Lerp Alpha" (Math|Float|SelectFloat 1.0 0.0 (and (Variables|Default|GetPlayerIsOverlapping) (Variables|Default|GetisActive))) :!class /Script/Engine.MaterialInstanceDynamic)
        (if (and (Variables|Default|GetPlayerIsOverlapping) (Variables|Default|GetisActive))
          (for _index (range 0 (- (Utilities|Array|Length _blueprintstoalert) 1))
            (Class|AlarmInterface|SendAlarm(Message) (Utilities|Array|Get(acopy) _blueprintstoalert _index) true)))))))

(fn ConstructionScript
  (bind _returnvalue (Rendering|Material|CreateDynamicMaterialInstance (Variables|Default|GetPoseableMesh) 1 0 :!class /Script/Engine.PrimitiveComponent))
  (Variables|Default|SetDynMat _returnvalue)
  (Components|Timeline|SetPlayRate (Variables|Default|Getrotate%20camera) (Variables|Default|GetTurn%20speed)))