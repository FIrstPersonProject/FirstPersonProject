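; AlarmBox is an actor that gradually changes color while another actor overlaps it and fades back when the overlap ends.
; The construction script creates a dynamic material instance and resets the color value to its start.
; Overlap events toggle a proximity flag without filtering the other actor.
; Tick ramps the clamped value up or down over about one second and feeds it to the material's ColorChangeAmount parameter.
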(event EventBeginPlay)

(event EventActorBeginOverlap
  (params (OtherActor :type Actor%20Object%20Reference))
  (Variables|Default|SetIsNear true))

(event EventActorEndOverlap
  (params (OtherActor :type Actor%20Object%20Reference))
  (Variables|Default|SetIsNear false))

(event EventTick
  (params (DeltaSeconds :type Float%20%28single-precision%29))
  (Rendering|Material|SetScalarParameterValue (Variables|Default|GetDynamicMaterialRef) "ColorChangeAmount" (Variables|Default|GetColorValue) :!class /Script/Engine.MaterialInstanceDynamic)
  (if (Variables|Default|GetIsNear)
    (Variables|Default|SetColorValue (Math|Float|Clamp(Float) (+ (Variables|Default|GetColorValue) DeltaSeconds)))
    (else
      (Variables|Default|SetColorValue (Math|Float|Clamp(Float) (- (Variables|Default|GetColorValue) DeltaSeconds))))))

(fn ConstructionScript
  (bind _returnvalue (Rendering|Material|CreateDynamicMaterialInstance 0 "/Game/Materials/DynamicMaterial_Inst.DynamicMaterial_Inst" :!class /Script/Engine.PrimitiveComponent))
  (Variables|Default|SetDynamicMaterialRef _returnvalue)
  (bind _output_get (Variables|Default|SetStartValue 0.0))
  (Variables|Default|SetColorValue _output_get))