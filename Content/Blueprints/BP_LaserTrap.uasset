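; BP_LaserTrap is a laser trap that blinks on and off and raises an alarm while the player overlaps it.
; A looping timer toggles active state and visibility, using a first delay, then switching to a repeat interval.
; While active and overlapped, Tick turns the cube red and sends SendAlarmMessage every frame.
; Alerts reach either a configured local list or every AlarmInterface actor.
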(event Custom|ToggleActive
  (bind _output_get (Variables|Default|SetActive (not (stale _output_get))))
  (Rendering|SetVisibility _output_get false)
  (Utilities|Time|SetTimerbyFunctionName 0 "ToggleActive" (Variables|Default|GetdelayBetweenToggling) true))

(event EventBeginPlay
  (Utilities|Time|SetTimerbyFunctionName 0 "ToggleActive" (Variables|Default|GetdelayOnFirstTick) true)
  (bind _output_get (Variables|Default|SetActive (Variables|Default|GetActiveOnStart)))
  (Rendering|SetVisibility _output_get false))

(event EventActorBeginOverlap
  (params (OtherActor :type Actor%20Object%20Reference))
  (Variables|Default|SetisOverlapping (== OtherActor (Game|GetPlayerCharacter 0))))

(event EventTick
  (params (DeltaSeconds :type Float%20%28single-precision%29))
  (bind _blueprints_to_activate_on_local_alert (Variables|Default|GetBlueprints%20to%20activate%20on%20local%20alert))
  (if (and (Variables|Default|GetActive) (Variables|Default|GetisOverlapping))
    (Rendering|Material|SetMaterial (Variables|Default|GetCube) 0 "/Game/Materials/red_matte.red_matte")
    (if (Variables|Default|GetonlyLocalAlert)
      (for _index (range 0 (- (Utilities|Array|Length _blueprints_to_activate_on_local_alert) 1))
        (Class|AlarmInterface|SendAlarm(Message) (Utilities|Array|Get(acopy) _blueprints_to_activate_on_local_alert _index) true))
      (else
        (bind _outactors (Actor|GetAllActorswithInterface "/Game/AlarmInterface.AlarmInterface_C"))
        (for _index_2 (range 0 (- (Utilities|Array|Length _outactors) 1))
          (Class|AlarmInterface|SendAlarm(Message) (Utilities|Array|Get(acopy) _outactors _index_2) true))))
    (else
      (Rendering|Material|SetMaterial (Variables|Default|GetCube) 0 "/Game/FirstPersonBP/Meshes/CubeMaterial.CubeMaterial"))))

(event EventActorEndOverlap
  (params (OtherActor :type Actor%20Object%20Reference))
  (Variables|Default|SetisOverlapping false))

(fn ConstructionScript)