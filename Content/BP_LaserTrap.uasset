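; BP_LaserTrap is a laser trap actor that blinks on and off and signals when something overlaps it during its active phase.
; A looping one-second timer flips the Active flag and toggles the laser mesh's visibility.
; Actor overlap events set an IsOverlapping flag without filtering the other actor.
; Tick sets the Cube's material to red while both flags are true, otherwise to its default material.
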(event Custom|ToggleActive
  (bind _output_get (Variables|Default|SetActive (not (stale _output_get))))
  (Rendering|ToggleVisibility (Variables|Default|GetLaser_StaticMesh) false))

(event EventBeginPlay
  (Utilities|Time|SetTimerbyFunctionName 0 "ToggleActive" 1.0 true)
  (Variables|Default|SetActive true))

(event EventActorBeginOverlap
  (params (OtherActor :type Actor%20Object%20Reference))
  (Variables|Default|SetisOverlapping true))

(event EventTick
  (params (DeltaSeconds :type Float%20%28single-precision%29))
  (if (and (Variables|Default|GetActive) (Variables|Default|GetisOverlapping))
    (Rendering|Material|SetMaterial (Variables|Default|GetCube) 0 "/Game/red_matte.red_matte")
    (else
      (Rendering|Material|SetMaterial (Variables|Default|GetCube) 0 "/Game/FirstPersonBP/Meshes/CubeMaterial.CubeMaterial"))))

(event EventActorEndOverlap
  (params (OtherActor :type Actor%20Object%20Reference))
  (Variables|Default|SetisOverlapping false))

(fn ConstructionScript)